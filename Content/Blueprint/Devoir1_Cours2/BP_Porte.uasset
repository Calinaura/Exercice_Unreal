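; Door that toggles between open and closed by instantly moving its Cube to a lowered or raised relative position, with no animation.
; BeginPlay lowers the Cube when IsOpened is set by default.
; ActivateDoor calls OpenOrClose, which moves the Cube and flips IsOpened.
; Each toggle then calls VerificationDoorsClosed on BPLightDoors so the light can check the doors' state.
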(event `self.ReceiveBeginPlay`
  ;[0.375 0.375 0.375] Vérifie si les portes sont ouvertes ou fermées par défaut et les mets dans la bonne position
  (if (`self.IsOpened?`)
    (`SceneComponent.K2_SetRelativeLocation` (`self.Cube`) (0.0 0.0 -100.0) false false)))

(event `/Game/Blueprint/Devoir1_Cours2/BPI_Portes.ActivateDoor`
  ;[0 0.3073 0.04698] Si les portes sont activées alors ça lance l'ouverture ou la fermeture
  (`self.OpenOrClose`))

(event `OpenOrClose`
  ;[0.4271 0.2674 0] Vérifie si les portes sont ouvertes ou fermées
  (if (`self.IsOpened?`)
    ;[1 1 1] Change la position de la porte en "fermée"
    (`SceneComponent.K2_SetRelativeLocation` (`self.Cube`) (0.0 0.0 100.0) false false)
    (set `self.IsOpened?` false)
    (else
      ;[1 1 1] Change la position de la porte en "ouverte"
      (`SceneComponent.K2_SetRelativeLocation` (`self.Cube`) (0.0 0.0 -100.0) false false)
      (set `self.IsOpened?` true)))
  ;[0.00324 0.3177 0.3114] Lance la vérification pour la light afin de savoir si les portes sont ouvertes ou fermées
  (`/Game/Blueprint/Devoir1_Cours2/BP_LightDoors.VerificationDoorsClosed` (`self.BP_LightDoors`)))

(fn `UserConstructionScript`)