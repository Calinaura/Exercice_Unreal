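; BP_LightDoors is a status light that reflects whether three referenced doors are all closed and switches linked enemies on or off accordingly.
; Its VerificationDoorsClosed event reads each door's IsOpened flag.
; When all are closed, it turns the point light green and activates every valid enemy in the BPEnnemy array.
; Otherwise it turns the light red and deactivates them.
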(event `VerificationDoorsClosed`
  ;[0.401 0 0] Vérification pour savoir si TOUTES les portes sont fermées ou pas
  (if (and (not (`/Game/Blueprint/Devoir1_Cours2/BP_Porte.IsOpened?` (`self.Porte1`))) (not (`/Game/Blueprint/Devoir1_Cours2/BP_Porte.IsOpened?` (`self.Porte2`))) (not (`/Game/Blueprint/Devoir1_Cours2/BP_Porte.IsOpened?` (`self.Porte3`))))
    ;[0.0219 0.2552 0] Si les portes sont bien fermées alors ça change la couleur de la light et ça active les ennemis
    (`LightComponent.SetLightColor` (`self.PointLight`) (struct :`G` 1.0 :`B` 0.06906 :`A` 1.0) true)
    (for _array_element (`self.BP_Ennemy`)
      (`/Engine/EditorBlueprintResources/StandardMacros.IsValid` _array_element
        (:`Is Valid`
          (`/Game/Blueprint/Devoir1_Cours2/BPI_Ennemy.ActivateEnnemy` _array_element))))
    (else
      ;[0.3802 0.3269 0] Si les portes sont toujours ouvertes alors la light reste rouge et ça désactive les ennemis
      (`LightComponent.SetLightColor` (`self.PointLight`) (struct :`R` 1.0 :`A` 1.0) true)
      (for _array_element_2 (`self.BP_Ennemy`)
        (`/Engine/EditorBlueprintResources/StandardMacros.IsValid` _array_element_2
          (:`Is Valid`
            (`/Game/Blueprint/Devoir1_Cours2/BPI_Ennemy.DeactivateEnnemy` _array_element_2)))))))

(fn `UserConstructionScript`)