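; BP_PNJ is an NPC that wanders and shows quest dialogue to the player character.
; A looping AI MoveTo picks random reachable points within a radius, standing in for a behavior tree.
; Seeing the player through PawnSensing freezes it via CustomTimeDilation until a short, refreshable timer restores it.
; Box overlap creates a widget with text from Content indexed by the player's QuestAdvance, collapsed on exit.
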(event `self.ReceiveBeginPlay`
  ;[1 1 1] IA (j'arrivais pas à faire de behavior tree qui fonctionne :( )
  (`self.patrol`))

(event `Patrol`
  ;[1 1 1] IA (j'arrivais pas à faire de behavior tree qui fonctionne :( )
  (`|AIMoveTo` self (`NavigationSystemV1.K2_GetRandomReachablePointInRadius` (`SceneComponent.K2_GetComponentLocation` (`self.CapsuleComponent`)) 500.0 null null) null
    (:`OnSuccess`
      _)
    (:`OnFail`
      _))
  (`self.patrol`))

(event `self.PawnSensing.OnSeePawn`
  (params (Pawn :type "Pawn Object Reference"))
  ;[1 1 1] IA (j'arrivais pas à faire de behavior tree qui fonctionne :( )
  (cast `/Game/ThirdPerson/Blueprints/BP_ThirdPersonCharacter` Pawn)
  (`KismetSystemLibrary.K2_ClearAndInvalidateTimerHandle` (`self.Timer`))
  (set `self.CustomTimeDilation` 0.0)
  (bind _returnvalue (`KismetSystemLibrary.K2_SetTimerDelegate` (delegate `Restart patrol`) 3.0))
  (set `self.Timer` _returnvalue))

(event `Restart patrol`
  ;[1 1 1] IA (j'arrivais pas à faire de behavior tree qui fonctionne :( )
  (set `self.CustomTimeDilation` 1.0))

(event `self.Box.OnComponentBeginOverlap`
  (params (OverlappedComponent :type "PrimitiveComponent Object Reference") (OtherActor :type "Actor Object Reference") (OtherComp :type "PrimitiveComponent Object Reference") (OtherBodyIndex :type Integer) (bFromSweep :type Boolean) (SweepResult :type "HitResult Structure (by ref)"))
  ;[1 1 1] Dialogues du PNJ (déso si c'est pas ouf, j'ai tenté des trucs)
  (bind _asbp_third_person_character (cast `/Game/ThirdPerson/Blueprints/BP_ThirdPersonCharacter` OtherActor))
  (bind _returnvalue (`|CreateWidget` "/Game/Blueprint/Devoir2_Cours3_4/Roxane/WB_Quest.WB_Quest_C"))
  (set `self.Widget` _returnvalue)
  (set `/Game/Blueprint/Devoir2_Cours3_4/Roxane/WB_Quest. Text` (`|GetArrayItem` (`self.Content`) (`/Game/ThirdPerson/Blueprints/BP_ThirdPersonCharacter.Quest_advance` _asbp_third_person_character)) _returnvalue)
  (`UserWidget.AddToViewport` (`self.Widget`) 0))

(event `self.Box.OnComponentEndOverlap`
  (params (OverlappedComponent :type "PrimitiveComponent Object Reference") (OtherActor :type "Actor Object Reference") (OtherComp :type "PrimitiveComponent Object Reference") (OtherBodyIndex :type Integer))
  ;[1 1 1] Dialogues du PNJ (déso si c'est pas ouf, j'ai tenté des trucs)
  (cast `/Game/ThirdPerson/Blueprints/BP_ThirdPersonCharacter` OtherActor)
  (`Widget.SetVisibility` (`self.Widget`) "Collapsed"))

(fn `UserConstructionScript`)