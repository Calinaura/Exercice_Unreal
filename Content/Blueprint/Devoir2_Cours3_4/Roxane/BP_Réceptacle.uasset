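; BP_Réceptacle is a quest receptacle where the player deposits the object they carry.
; When a BP_ThirdPersonCharacter overlaps the Box, it spawns that character's ObjectSaved class at the Sphere's transform, then clears ObjectSaved.
; The receptacle's GoodOne flag, not the object itself, decides the result: QuestAdvance becomes 2 if true, otherwise 1 unless it is already 2.
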(event `self.Box.OnComponentBeginOverlap`
  (params (OverlappedComponent :type "PrimitiveComponent Object Reference") (OtherActor :type "Actor Object Reference") (OtherComp :type "PrimitiveComponent Object Reference") (OtherBodyIndex :type Integer) (bFromSweep :type Boolean) (SweepResult :type "HitResult Structure (by ref)"))
  (bind _as_bp_third_person_character (`self.As BP Third Person Character`))
  (bind _as_bp_third_person_character_2 (`self.As BP Third Person Character`))
  ;[1 1 1] Spawn de l'objet et vérifie que c'est le bon
  (bind _asbp_third_person_character (cast `/Game/ThirdPerson/Blueprints/BP_ThirdPersonCharacter` OtherActor))
  (set `self.As BP Third Person Character` _asbp_third_person_character)
  (`|SpawnActorFromClass` (`/Game/ThirdPerson/Blueprints/BP_ThirdPersonCharacter.Object_saved` _as_bp_third_person_character) (`SceneComponent.K2_GetComponentToWorld` (`self.Sphere`)) "Undefined" "MultiplyWithRoot" null null)
  (set `/Game/ThirdPerson/Blueprints/BP_ThirdPersonCharacter.Object_saved` null _as_bp_third_person_character)
  (if (`self.Good_One?`)
    (set `/Game/ThirdPerson/Blueprints/BP_ThirdPersonCharacter.Quest_advance` 2 (`self.As BP Third Person Character`))
    (elif (not (== (`/Game/ThirdPerson/Blueprints/BP_ThirdPersonCharacter.Quest_advance` _as_bp_third_person_character_2) 2))
      (set `/Game/ThirdPerson/Blueprints/BP_ThirdPersonCharacter.Quest_advance` 1 _as_bp_third_person_character_2))))

(fn `UserConstructionScript`)