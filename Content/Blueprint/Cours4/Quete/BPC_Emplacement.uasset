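; Battery slot component for a quest generator, marking a location where a battery is placed.
; InsertObject stores the battery, disables collision on its box and moves it to the component's world location.
; It then casts its owner to BP_Generator and asks it to check this slot, printing a success message and triggering the generator's overall check when the slot is valid.
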(fn `InsertObject`
  (params (NewBattery :type "/Game/Blueprint/Cours4/Quete/BP_Battery Object Reference"))
  (locals (Generator :type "/Game/Blueprint/Cours4/Quete/BP_Generator Object Reference"))
  (bind _output_get (set `self.Battery` NewBattery))
  (`PrimitiveComponent.SetCollisionEnabled` (`/Game/Blueprint/Cours4/Quete/BP_Battery.Box` _output_get) "NoCollision")
  (`Actor.K2_SetActorLocation` _output_get (`self.K2_GetComponentLocation`) false false)
  (bind _asbp_generator (cast `/Game/Blueprint/Cours4/Quete/BP_Generator` (`self.GetOwner`)))
  (bind _output_get_2 (set `local.Generator` _asbp_generator))
  (bind _result (`/Game/Blueprint/Cours4/Quete/BP_Generator.CheckEmplacement` _output_get_2 self))
  (if _result
    (`KismetSystemLibrary.PrintString` "Bien joué !")
    (`/Game/Blueprint/Cours4/Quete/BP_Generator.CheckGenerator` (`local.Generator`))))