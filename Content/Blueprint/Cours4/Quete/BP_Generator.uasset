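; BP_Generator is a quest puzzle actor that verifies whether batteries of the right colors sit in its red, green and blue emplacements.
; On BeginPlay it gathers the three emplacements into an array, and CompareColor matches each slot's battery against the Solution array by index.
; CheckGenerator requires every slot to match, then signals the enigma solved and finishes the associated quest, otherwise signaling it lost.
; CheckEmplacement's branch ignores its color comparison result.
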(event `self.ReceiveBeginPlay`
  (`self.GetEmplacements`))

(fn `CheckEmplacement`
  (params (EmplacementToCheck :type "/Game/Blueprint/Cours4/Quete/BPC_Emplacement Object Reference"))
  (returns (Result :type Boolean))
  (locals (TempResult :type Boolean))
  (for _index (range (`KismetArrayLibrary.Array_Length` (`self.Emplacement`)))
    (if (== (`|GetArrayItem` (`self.Emplacement`) _index) EmplacementToCheck)
      (`self.CompareColor` 0)
      (if true
        (set `local.TempResult` true)
        (break)
        (else
          _)))
    (set `local.TempResult` false))
  (return (`local.TempResult`)))

(fn `CheckGenerator`
  (locals (Result :type Boolean))
  (bind _associatequest (`self.AssociateQuest`))
  (set `local.Result` true)
  (for _index (range (`KismetArrayLibrary.Array_Length` (`self.Emplacement`)))
    (bind _result (`self.CompareColor` _index))
    (if (not _result)
      (set `local.Result` false)
      (break)))
  (if (`local.Result`)
    (`self.OnEnigmeSolved`)
    (set `/Game/Blueprint/Cours4/Quete/BP_Quest.IsFinished` true _associatequest)
    (`/Game/Blueprint/Cours4/Quete/BP_Quest.FinishTheQuest` _associatequest)
    (else
      (`self.OnEnigmeLost`))))

(fn `CompareColor`
  (params (Index :type Integer))
  (returns (Result :type Boolean))
  (locals (TempResult :type Boolean))
  (bind _battery (`/Game/Blueprint/Cours4/Quete/BPC_Emplacement.Battery` (`|GetArrayItem` (`self.Emplacement`) Index)))
  (`/Engine/EditorBlueprintResources/StandardMacros.IsValid` _battery
    (:`Is Valid`
      (if (`|EnumEquality` (`/Game/Blueprint/Cours4/Quete/BP_Battery.BatteryColor` _battery) (`|GetArrayItem` (`self.Solution`) Index))
        (set `local.TempResult` true)
        (else
          (set `local.TempResult` false :!label _label))))
    (:`Is Not Valid`
      (goto _label)))
  (return (`local.TempResult`)))

(fn `GetEmplacements`
  (`|ExecutionSequence`
    (:`then_0`
      (`KismetArrayLibrary.Array_Add` (`self.Emplacement`) (`self.Red`)))
    (:`then_1`
      (`KismetArrayLibrary.Array_Add` (`self.Emplacement`) (`self.Green`)))
    (:`then_2`
      (`KismetArrayLibrary.Array_Add` (`self.Emplacement`) (`self.Blue`)))))

(fn `UserConstructionScript`)