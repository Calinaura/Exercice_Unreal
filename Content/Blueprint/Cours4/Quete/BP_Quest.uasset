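; BP_Quest is a quest Blueprint that tracks a ToDoList of items and reports completion up a chain.
; CheckQuestProgress scans the list for unfinished entries, but sets IsFinished false beforehand and never true, so as written it never reaches FinishTheQuest.
; FinishTheQuest asks a valid Referent to recheck its progress, otherwise it fires OnQuestFinished.
; BeginPlay binds that dispatcher to an empty placeholder event.
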(event `self.ReceiveBeginPlay`
  (add `self.OnQuestFinished` (delegate `oui`)))

(event `oui`)

(fn `CheckQuestProgress`
  (set `self.IsFinished` false)
  (for _index (range (`KismetArrayLibrary.Array_Length` (`self.ToDoList`)))
    (if (not (`/Game/Blueprint/Cours4/Quete/BP_Quest.IsFinished` (`|GetArrayItem` (`self.ToDoList`) _index)))
      (set `self.IsFinished` false)
      (break)))
  (if (`self.IsFinished`)
    (`self.FinishTheQuest`))
  (return))

(fn `FinishTheQuest`
  (bind _referent (`self.Referent`))
  (`/Engine/EditorBlueprintResources/StandardMacros.IsValid` _referent
    (:`Is Valid`
      (`self.CheckQuestProgress` _referent))
    (:`Is Not Valid`
      (`self.OnQuestFinished`))))

(fn `UserConstructionScript`)