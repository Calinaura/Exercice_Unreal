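; BP_Battery is a colored battery pickup that completes its associated quest when taken.
; The construction script creates a dynamic material on the cylinder, which BeginPlay tints blue, red or green from the BatteryColor variable.
; The Take event marks the quest finished, calls its finish function, then hides the battery by moving it far below and disabling collision instead of destroying it.
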(event `self.ReceiveBeginPlay`
  (`self.ChangeBatteryColor`))

(event `/Game/Blueprint/Cours4/Quete/BPI_ITransportable.Take`
  (bind _associatequest (`self.AssociateQuest`))
  (set `/Game/Blueprint/Cours4/Quete/BP_Quest.IsFinished` true _associatequest)
  (`/Game/Blueprint/Cours4/Quete/BP_Quest.FinishTheQuest` _associatequest)
  (`self.K2_SetActorLocation` (0.0 0.0 -1000.0))
  (`PrimitiveComponent.SetCollisionEnabled` (`self.Box`) "NoCollision")
  (`PrimitiveComponent.SetCollisionEnabled` (`self.Cylinder`) "NoCollision"))

(fn `ChangeBatteryColor`
  (switch `/Game/Blueprint/Cours4/Quete/BPE_BatteryColor` (`self.BatteryColor`)
    (:`NewEnumerator0`
      (`MaterialInstanceDynamic.SetVectorParameterValue` (`self.Material`) "AlbedoColor" (struct :`R` 0.040927 :`B` 1.0 :`A` 1.0)))
    (:`NewEnumerator1`
      (`MaterialInstanceDynamic.SetVectorParameterValue` (`self.Material`) "AlbedoColor" (struct :`R` 0.816667 :`B` 0.017654 :`A` 1.0)))
    (:`NewEnumerator2`
      (`MaterialInstanceDynamic.SetVectorParameterValue` (`self.Material`) "AlbedoColor" (struct :`G` 0.592 :`A` 1.0)))))

(fn `UserConstructionScript`
  (bind _returnvalue (`PrimitiveComponent.CreateDynamicMaterialInstance` (`self.Cylinder`) 0 "/Game/Blueprint/Cours4/Quete/Materials/MI_Battery.MI_Battery" "None"))
  (set `self.Material` _returnvalue))